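; BP_Mission is an actor that holds the runtime data of one mission: its info, owning player character, state and phase.
; Init stores the info and owner and resets the phase to zero.
; UpdateState and UpdatePhase print an on-screen debug message, store the new value and fire change dispatchers that pass the mission itself.
; It has no event logic, so changes come through these function calls.
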(fn `init`
  (params (InMissionInfo :type "/Game/MissionSystem/Mission_Info Structure") (InPlayerCharacter :type "/Game/ThirdPerson/Blueprints/BP_ThirdPersonCharacter Object Reference"))
  (set `self.Info` InMissionInfo)
  (set `self.OwnerPlayerCharacter` InPlayerCharacter)
  (set `self.Phase` 0))

(fn `updatePhase`
  (params (InNewPhase :type Integer))
  (bind (_info_name _info_numphases _info_nameui) (break `/Game/MissionSystem/Mission_Info` (`self.Info`)))
  (`KismetSystemLibrary.PrintString` (`KismetStringLibrary.Concat_StrStr` _info_nameui " " "Changet phase to '" (`KismetStringLibrary.Conv_IntToString` (`local.InNewPhase`)) "'") true true (struct :`G` 0.66 :`B` 1.0 :`A` 1.0) 1.0)
  (bind _output_get (set `self.Phase` (`local.InNewPhase`)))
  (`self.OnChangedPhaseMission` self _output_get))

(fn `updateState`
  (params (InNewState :type "/Game/MissionSystem/Enum_MissionState Enum" :default "NewEnumerator0"))
  (bind (_info_name _info_numphases _info_nameui) (break `/Game/MissionSystem/Mission_Info` (`self.Info`)))
  (`KismetSystemLibrary.PrintString` (`KismetStringLibrary.Concat_StrStr` "Задание '" _info_nameui "' изменено на '" (`|GetEnumeratorNameAsString` (`local.InNewState`)) "'") true true (struct :`G` 0.66 :`B` 1.0 :`A` 1.0) 5.0)
  (bind _output_get (set `self.State` (`local.InNewState`)))
  (`self.OnChangedStateMission` self _output_get))

(fn `UserConstructionScript`)