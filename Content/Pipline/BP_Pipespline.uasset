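; BP_Pipespline is an unfinished spline-based pipe actor whose construction script is meant to build spline mesh segments along a Spline component.
; The loop adds SplineMeshComponents and sets their forward axis to Y, but its last index is not connected.
; The point-count calculation and the SetStartAndEnd call that fits each segment between neighboring spline points sit unwired, so neither runs.
; The event graph holds only disabled default events.
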(event EventBeginPlay)

(event Collision|EventActorBeginOverlap
  (params (OtherActor :type Actor%20Object%20Reference)))

(event EventTick
  (params (DeltaSeconds :type Float%20%28single-precision%29)))

(fn ConstructionScript
  (for _index (range 0 (stale _result))
    (bind _returnvalue (AddComponent|AddSplineMeshComponent false))
    (SplineMesh|SetForwardAxis _returnvalue "Y" true)))