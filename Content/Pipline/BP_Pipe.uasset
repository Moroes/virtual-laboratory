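; BP_Pipe is an interactable pipe whose valve component (Ventyl) turns when the player uses it.
; Interacte calls Rotate, where a FlipFlop alternates quarter turns in opposite directions, animated by MoveComponentTo relative to the valve's current rotation.
; PreInteracte returns a Russian "Press E to interact" prompt.
; The turn is purely a rotation, with no flow or puzzle state in this Blueprint.
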(event `Rotate`
  (bind _ventyl (`self.Ventyl`))
  (bind _relativelocation (`SceneComponent.RelativeLocation` _ventyl))
  (bind _relativerotation (`SceneComponent.RelativeRotation` _ventyl))
  (`/Engine/EditorBlueprintResources/StandardMacros.FlipFlop`
    (:`A`
      (`KismetSystemLibrary.MoveComponentTo` (`self.Ventyl`) _relativelocation (`KismetMathLibrary.NormalizedDeltaRotator` _relativerotation (struct :`Yaw` 90.0)) false false 1.0))
    (:`B`
      (`KismetSystemLibrary.MoveComponentTo` (`self.Ventyl`) _relativelocation (`KismetMathLibrary.NormalizedDeltaRotator` _relativerotation (struct :`Yaw` -90.0)) false false 1.0))))

(event `/Game/Light/I_Inter.Interacte`
  (`self.Rotate`))

(fn `Pre Interacte`
  (returns (NewParam :type String))
  (return "Нажмите E для взаимодействия"))

(fn `UserConstructionScript`)