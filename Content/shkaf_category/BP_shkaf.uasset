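; Interactable cabinet (shkaf) with a swinging right protective glass and an inspection (osmotr) task tied to the player's mission.
; Interacting alternately rotates the glass 90 degrees one way and back over a second, using a FlipFlop and MoveComponentTo.
; check_shkaf marks inspection points in a boolean array; once all are set, it latches completion and updates the current mission's state through the player character's MissionManager.
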(event `self.ReceiveBeginPlay`)

(event `check_shkaf`
  (params (number :type Integer))
  (bind _osmotr (`self.osmotr`))
  (`KismetArrayLibrary.Array_Set` _osmotr number true)
  (for _array_element _osmotr
    (if _array_element
      (set `self.osmotr_flag` true)
      (else
        (set `self.osmotr_flag` false)
        (break))))
  (if (== (`self.osmotr_flag`) (not (`self.complet_osmotr`)))
    (set `self.complet_osmotr` true)
    (`self.completed_osmotr`)))

(event `completed_osmotr`
  (bind _asbp_third_person_character (cast `/Game/ThirdPerson/Blueprints/BP_ThirdPersonCharacter` (`GameplayStatics.GetPlayerCharacter` 0)))
  (`/Game/MissionSystem/BP_Mission.updateState` (`/Game/MissionSystem/BP_MissionManager.CurrentMission` (`/Game/ThirdPerson/Blueprints/BP_ThirdPersonCharacter.MissionManager` _asbp_third_person_character)) "NewEnumerator2"))

(event `rotate_glass`
  (bind `_shkaf_правое_защитное_стекло` (`self.shkaf_Правое_защитное_стекло`))
  (bind _relativelocation (`SceneComponent.RelativeLocation` `_shkaf_правое_защитное_стекло`))
  (bind _relativerotation (`SceneComponent.RelativeRotation` `_shkaf_правое_защитное_стекло`))
  (`/Engine/EditorBlueprintResources/StandardMacros.FlipFlop`
    (:`A`
      (`KismetSystemLibrary.MoveComponentTo` (`self.shkaf_Правое_защитное_стекло`) _relativelocation (`KismetMathLibrary.NormalizedDeltaRotator` _relativerotation (struct :`Roll` 90.0)) false false 1.0))
    (:`B`
      (`KismetSystemLibrary.MoveComponentTo` (`self.shkaf_Правое_защитное_стекло`) _relativelocation (`KismetMathLibrary.NormalizedDeltaRotator` _relativerotation (struct :`Roll` -90.0)) false false 1.0))))

(event `/Game/Light/I_Inter.Interacte`
  (`self.rotate_glass`))

(fn `Pre Interacte`
  (returns (NewParam :type String))
  (return ""))

(fn `UserConstructionScript`)